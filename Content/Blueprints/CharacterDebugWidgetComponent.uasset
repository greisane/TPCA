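; Widget component that keeps a character debug widget positioned at the top of its owning Character's capsule.
; On BeginPlay it caches the owner and capsule height, then switches to absolute location.
; Each tick it follows the capsule's base plus an interpolated height.
; Interpolating height rather than position smooths crouch and stand transitions while jumps and falls are tracked without lag.
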(event `self.ReceiveBeginPlay`
  ;[0 0 0 1 12] Setup Character Reference
  (bind _ascharacter (cast `Character` (`self.GetOwner`)))
  (bind _output_get (set `self.CharacterOwner` _ascharacter))
  (bind _capsulecomponent (`Character.CapsuleComponent` _output_get))
  (bind _returnvalue (`CapsuleComponent.GetScaledCapsuleHalfHeight` _capsulecomponent))
  ;[0 0 0 1 12] Initialize Variables
  (set `self.Height` (* _returnvalue 2.0))
  ;[0 0 0 1 12] Set initial location above the character
  (`self.SetAbsolute` true)
  (bind (_returnvalue_x _returnvalue_y _returnvalue_z) (`KismetMathLibrary.BreakVector` (`self.K2_GetComponentLocation` _capsulecomponent)))
  (`self.K2_SetWorldLocation` (`KismetMathLibrary.MakeVector` _returnvalue_x _returnvalue_y (+ _returnvalue_z _returnvalue))))

(event `self.ReceiveTick`
  (params (DeltaSeconds :type "Float (single-precision)"))
  (bind _characterowner (`self.CharacterOwner`))
  (bind _capsulecomponent (`Character.CapsuleComponent` _characterowner))
  (bind _returnvalue (`CapsuleComponent.GetScaledCapsuleHalfHeight` _capsulecomponent))
  (bind (_returnvalue_x _returnvalue_y _returnvalue_z) (`KismetMathLibrary.BreakVector` (`self.K2_GetComponentLocation` _capsulecomponent)))
  ;[0 0 0 1 12] To have the text smoothly move when we crouch/stand but not in other cases (when we fall of jump for instance) we have to interpolate the desired height instead of the position directly
  (`/Engine/EditorBlueprintResources/StandardMacros.IsValid` _characterowner
    (:`Is Valid`
      (bind _output_get (set `self.Height` (`KismetMathLibrary.FInterpTo` (stale _output_get) (* _returnvalue 2.0) DeltaSeconds 5.0)))
      (`self.K2_SetWorldLocation` (`KismetMathLibrary.MakeVector` _returnvalue_x _returnvalue_y (+ _output_get (- _returnvalue_z _returnvalue)))))))